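; BP_Lane_Water is a water lane Blueprint that carries the player along and kills them on contact with its lane meshes.
; While the living player overlaps PlayerTriggerZone, Tick shifts their TargetLocation along Y by VehicleSpeed scaled by frame time.
; Overlap or hit events on the three lane meshes cast to BP_Player and call DeathReset.
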(event OnComponentBeginOverlap(LaneMesh)
  (params (OverlappedComponent :type Primitive%20Component%20Object%20Reference) (OtherActor :type Actor%20Object%20Reference) (OtherComp :type Primitive%20Component%20Object%20Reference) (OtherBodyIndex :type Integer) (bFromSweep :type Boolean) (SweepResult :type Hit%20Result%20Structure%20%28by%20ref%29))
  (bind _asbp_player (Utilities|Casting|CastToBP_Player OtherActor))
  (Default|DeathReset _asbp_player))

(event OnComponentBeginOverlap(LaneMesh1)
  (params (OverlappedComponent :type Primitive%20Component%20Object%20Reference) (OtherActor :type Actor%20Object%20Reference) (OtherComp :type Primitive%20Component%20Object%20Reference) (OtherBodyIndex :type Integer) (bFromSweep :type Boolean) (SweepResult :type Hit%20Result%20Structure%20%28by%20ref%29))
  (bind _asbp_player (Utilities|Casting|CastToBP_Player OtherActor))
  (Default|DeathReset _asbp_player))

(event OnComponentHit(LaneMesh)
  (params (HitComponent :type Primitive%20Component%20Object%20Reference) (OtherActor :type Actor%20Object%20Reference) (OtherComp :type Primitive%20Component%20Object%20Reference) (NormalImpulse :type Vector :default "0, 0, 0") (Hit :type Hit%20Result%20Structure%20%28by%20ref%29))
  (bind _asbp_player (Utilities|Casting|CastToBP_Player (stale OnComponentBeginOverlap(LaneMesh) OtherActor)))
  (Default|DeathReset _asbp_player))

(event OnComponentHit(LaneMesh1)
  (params (HitComponent :type Primitive%20Component%20Object%20Reference) (OtherActor :type Actor%20Object%20Reference) (OtherComp :type Primitive%20Component%20Object%20Reference) (NormalImpulse :type Vector :default "0, 0, 0") (Hit :type Hit%20Result%20Structure%20%28by%20ref%29))
  (bind _asbp_player (Utilities|Casting|CastToBP_Player (stale OnComponentBeginOverlap(LaneMesh1) OtherActor)))
  (Default|DeathReset _asbp_player))

(event OnComponentHit(LaneMesh2)
  (params (HitComponent :type Primitive%20Component%20Object%20Reference) (OtherActor :type Actor%20Object%20Reference) (OtherComp :type Primitive%20Component%20Object%20Reference) (NormalImpulse :type Vector :default "0, 0, 0") (Hit :type Hit%20Result%20Structure%20%28by%20ref%29))
  (bind _asbp_player (Utilities|Casting|CastToBP_Player (stale OnComponentBeginOverlap(LaneMesh2) OtherActor)))
  (Default|DeathReset _asbp_player))

(event OnComponentBeginOverlap(LaneMesh2)
  (params (OverlappedComponent :type Primitive%20Component%20Object%20Reference) (OtherActor :type Actor%20Object%20Reference) (OtherComp :type Primitive%20Component%20Object%20Reference) (OtherBodyIndex :type Integer) (bFromSweep :type Boolean) (SweepResult :type Hit%20Result%20Structure%20%28by%20ref%29))
  (bind _asbp_player (Utilities|Casting|CastToBP_Player OtherActor))
  (Default|DeathReset _asbp_player))

(event EventBeginPlay
  (|CallParentFunction) ; This node is disabled and will not be called.\nDrag off pins to build functionality.
)

(event Collision|EventActorBeginOverlap
  (params (OtherActor :type Actor%20Object%20Reference))
  (|CallParentFunction OtherActor) ; This node is disabled and will not be called.\nDrag off pins to build functionality.
)

(event EventTick
  (params (DeltaSeconds :type Float%20%28single-precision%29))
  (bind _returnvalue (Game|GetPlayerCharacter 0))
  (|CallParentFunction DeltaSeconds)
  (bind _asbp_player (Utilities|Casting|CastToBP_Player _returnvalue))
  (if (and (Collision|IsOverlappingActor (Variables|Default|GetPlayerTriggerZone) _returnvalue :!class /Script/Engine.PrimitiveComponent) (not (Variables|/Game/Blueprints/BP_Player.BP_Player_C|GetIsDead _asbp_player)))
    (Variables|/Game/Blueprints/BP_Player.BP_Player_C|SetTargetLocation _asbp_player (+ (Math|Vector|MakeVector 0.0 (* (Variables|Default|GetVehicleSpeed) DeltaSeconds) 0.0) (Variables|/Game/Blueprints/BP_Player.BP_Player_C|GetTargetLocation _asbp_player)))))

(fn ConstructionScript
  (|CallParentFunction))