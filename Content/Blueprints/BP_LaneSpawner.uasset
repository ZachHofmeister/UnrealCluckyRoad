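; Lane spawner that builds a chained strip of lanes, seeding safe lanes from behind the player at BeginPlay, then randomly chosen ones.
; Each lane attaches at the newest lane's spawn point, receives a spawner reference, and is reversed on even counts.
; Lane types run in random-length streaks of safe or obstacle lanes, with safe variants cycled by lane count.
; The oldest lane is destroyed once the list exceeds its cap.
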(event EventBeginPlay
  (CallFunction|SpawnInitialLanes))

(event Collision|EventActorBeginOverlap
  (params (OtherActor :type Actor%20Object%20Reference)))

(event EventTick
  (params (DeltaSeconds :type Float%20%28single-precision%29)))

(fn ConstructionScript)

(fn SpawnInitialLanes
  (Utilities|FlowControl|Sequence
    (:then_0
      (for _index (range 0 8)
        (bind _safe_lane (CallFunction|ChooseSafeLaneType))
        (Utilities|IsValid (Variables|Default|GetNewestLane)
          (:Is%20Valid
            (CallFunction|SpawnLaneatSpawnPoint _safe_lane)
            (Variables|/Game/Blueprints/Lanes/BP_Lane.BP_Lane_C|SetTraveled (Variables|Default|GetNewestLane) true))
          (:Is%20Not%20Valid
            (bind _asbp_player (Utilities|Casting|CastToBP_Player (Game|Player|GetPlayerPawn 0)))
            (CallFunction|SpawnLane _safe_lane (+ (Transformation|GetWorldLocation (Variables|/Game/Blueprints/BP_Player.BP_Player_C|GetLaneSpawn _asbp_player)) (Math|Vector|MakeVector (* -5.0 8e+01) 0.0 0.0)))
            (Variables|/Game/Blueprints/Lanes/BP_Lane.BP_Lane_C|SetTraveled (Variables|Default|GetNewestLane) true)))))
    (:then_1
      (for _index_2 (range 0 17)
        (CallFunction|SpawnLaneatSpawnPoint)))))

(fn SpawnLane
  (params (Lane%20Type :type BP%20Lane%20Class%20Reference) (SpawnLocation :type Vector))
  (if (Utilities|IsValidClass Lane%20Type)
    (LocalVariables|SetSpawnLaneType Lane%20Type)
    (else
      (bind _chosen_lane (CallFunction|ChooseLaneType))
      (LocalVariables|SetSpawnLaneType _chosen_lane)))
  (bind _returnvalue (Game|SpawnActorfromClass (LocalVariables|GetSpawnLaneType) (Math|Transform|MakeTransform SpawnLocation "0, 0, 0" "1,1,1") "Undefined" 0 0))
  (bind _output_get (Variables|Default|SetNewestLane _returnvalue))
  (Variables|/Game/Blueprints/Lanes/BP_Lane.BP_Lane_C|SetLaneSpawner _output_get self)
  (bind _iseven (CallFunction|IsLaneCountEven))
  (if _iseven
    (Default|ReverseLane _output_get))
  (Utilities|Array|Add (Variables|Default|GetLanes) _output_get)
  (Math|Integer|IncrementInt (Variables|Default|GetLaneCount)
    (:%20%20
      (CallFunction|CullMaxLanes))))

(fn SpawnLaneatSpawnPoint
  (params (Lane%20Type :type BP%20Lane%20Class%20Reference))
  (CallFunction|SpawnLane Lane%20Type (Transformation|GetWorldLocation (Variables|/Game/Blueprints/Lanes/BP_Lane.BP_Lane_C|GetLaneSpawnPoint (Variables|Default|GetNewestLane)))))

(fn ChooseLaneType
  (if (and (> (Variables|Default|GetLaneTypeRemaining) 0) (Utilities|IsValidClass (Variables|Default|GetCurrentLaneType)))
    _
    (else
      (Variables|Default|SetLaneTypeRemaining (Math|Random|RandomIntegerinRange (Variables|Default|GetMinLaneRemaining) (Variables|Default|GetMaxLaneRemaining)))
      (if (or (<= (Math|Random|RandomFloat) (Variables|Default|GetObstacleLaneChance)) (Utilities|Array|ContainsItem (Variables|Default|GetSafeLaneTypes) (Variables|Default|GetCurrentLaneType)))
        (bind _lanesexcept (CallFunction|GetLanesExcept (Variables|Default|GetObstacleLaneTypes) (Variables|Default|GetCurrentLaneType)))
        (Variables|Default|SetCurrentLaneType (.OutItem (Utilities|Array|Random _lanesexcept)))
        (else
          (Variables|Default|SetCurrentLaneType "/Game/Blueprints/Lanes/BP_Lane.BP_Lane_C")))))
  (Math|Integer|DecrementInt (Variables|Default|GetLaneTypeRemaining)
    (:%20%20
      (Utilities|FlowControl|Sequence
        (:then_0
          (if (Utilities|Array|ContainsItem (Variables|Default|GetSafeLaneTypes) (Variables|Default|GetCurrentLaneType))
            (bind _safe_lane (CallFunction|ChooseSafeLaneType))
            (Variables|Default|SetCurrentLaneType _safe_lane)))
        (:then_1
          (return (Variables|Default|GetCurrentLaneType)))))))

(fn CullMaxLanes
  (bind _lanes (Variables|Default|GetLanes))
  (if (not (<= (Utilities|Array|Length _lanes) (Variables|Default|GetMaxLanesAllowed)))
    (bind _output_get (LocalVariables|SetLaneToDel (Utilities|Array|Get(acopy) _lanes)))
    (Utilities|Array|RemoveIndex _lanes)
    (Default|DestroyLane _output_get)))

(fn IsLaneCountEven
  (return (== (Math|Integer|%(Integer) (Variables|Default|GetLaneCount) 2) 0)))

(fn ChooseSafeLaneType
  (bind _safelanetypes (Variables|Default|GetSafeLaneTypes))
  (return (Utilities|Array|Get(acopy) _safelanetypes (Math|Integer|%(Integer) (Variables|Default|GetLaneCount) (Utilities|Array|Length _safelanetypes)))))

(fn GetLanesExcept
  (params (In :type Array%20of%20BP%20Lane%20Class%20References) (Except :type BP%20Lane%20Class%20Reference))
  (for _array_element In
    (if (not (== _array_element Except))
      (Utilities|Array|Add (LocalVariables|GetReturnArray) _array_element)))
  (return (LocalVariables|GetReturnArray)))