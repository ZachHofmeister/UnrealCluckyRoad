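; Player character for a Crossy Road-style game, hopping a chicken mesh (Clucky) around while tracking score and coins in a Score widget.
; Axis input sets facing and, unless a line trace hits BP_Decor, shifts the target and launches a jump when grounded; Tick interpolates toward both.
; Overlapping a deadly BP_Car plays a timeline-driven scale animation and reloads the level after a delay.
; The MoveDelay cooldown call is disconnected.
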(event OnComponentBeginOverlap(CapsuleComponent)
  (params (OverlappedComponent :type Primitive%20Component%20Object%20Reference) (OtherActor :type Actor%20Object%20Reference) (OtherComp :type Primitive%20Component%20Object%20Reference) (OtherBodyIndex :type Integer) (bFromSweep :type Boolean) (SweepResult :type Hit%20Result%20Structure%20%28by%20ref%29))
  (bind _asbp_car (Utilities|Casting|CastToBP_Car OtherActor))
  (if (Variables|/Game/Blueprints/Cars/BP_Car.BP_Car_C|Getdeadly _asbp_car)
    (CallFunction|DeathReset)))

(event Custom|MoveDelay
  (Utilities|FlowControl|DoOnce false :!label _label
    (:Completed
      (Variables|Default|SetCanMove false)
      (Utilities|FlowControl|Delay (Variables|Default|GetMoveDelayTime))
      (Variables|Default|SetCanMove true)
      (goto _label Reset))))

(event Custom|DeathReset
  (Variables|Default|SetIsDead true)
  (Utilities|FlowControl|Delay 1.5)
  (bind _returnvalue (Game|GetCurrentLevelName true))
  (Game|OpenLevel(byName) (Utilities|String|StringToName _returnvalue)))

(event EventBeginPlay
  (Variables|Default|SetTargetLocation (Transformation|GetActorLocation))
  (bind _returnvalue (UserInterface|CreateWidget "/Game/Blueprints/UI/Score.Score_C"))
  (bind _output_get (Variables|Default|SetScoreUI _returnvalue))
  (UserInterface|Viewport|AddtoViewport _output_get 0))

(event Collision|EventActorBeginOverlap
  (params (OtherActor :type Actor%20Object%20Reference)))

(event EventTick
  (params (DeltaSeconds :type Float%20%28single-precision%29))
  (bind _clucky (Variables|Default|GetClucky))
  (Utilities|FlowControl|Sequence
    (:then_0
      (CallFunction|UpdateGrounded))
    (:then_1
      (Components|MoveComponentTo (Variables|Transformation|GetRootComponent) (Variables|Default|GetTargetLocation) "0, 0, 0" false false (Variables|Default|GetMoveDelayTime) false))
    (:then_2
      (Components|MoveComponentTo _clucky (Variables|/Script/Engine.SceneComponent|GetRelativeLocation _clucky) (Variables|Default|GetTargetRotation) false false (Variables|Default|GetMoveDelayTime) false))
    (:then_3
      (if (Variables|Default|GetIsDead)
        (bind _newtrack_0 (Timeline|Timeline_0 Play)
          (:Update
            (Transformation|SetRelativeScale3D (Variables|Default|GetClucky) _newtrack_0)))))))

(event Input|AxisEvents|InputAxisMoveVertical
  (params (AxisValue :type Float%20%28single-precision%29))
  (if (>= (Math|Float|Absolute(Float) AxisValue) 0.3)
    (Variables|Default|SetTargetRotation (Math|Rotator|MakeRotator 0.0 0.0 (Math|Float|SelectFloat 1.8e+02 0.0 (< AxisValue 0.0))))
    (CallFunction|TryMoveTimer (Math|Vector|MakeVector (* AxisValue 8e+01) 0.0 0.0))))

(event Input|AxisEvents|InputAxisMoveHorizontal
  (params (AxisValue :type Float%20%28single-precision%29))
  (if (>= (Math|Float|Absolute(Float) AxisValue) 0.3)
    (Variables|Default|SetTargetRotation (Math|Rotator|MakeRotator 0.0 0.0 (Math|Float|SelectFloat -9e+01 9e+01 (< AxisValue 0.0))))
    (CallFunction|TryMoveTimer (Math|Vector|MakeVector 0.0 (* AxisValue 8e+01) 0.0))))

(fn ConstructionScript)

(fn TryMoveTimer
  (params (Direction :type Vector))
  (bind _outhit (Collision|LineTraceForObjects (Transformation|GetActorLocation) (+ Direction (Variables|Default|GetTargetLocation)) (Utilities|Array|MakeArray "ObjectTypeQuery2") false 0 "None"))
  (if (.bBlockingHit (Collision|BreakHitResult _outhit))
    (Utilities|Casting|CastToBP_Decor (.HitActor (Collision|BreakHitResult _outhit))
      (:CastFailed
        _)))
  (if (and (Variables|Default|GetCanMove) (Variables|Default|GetIsGrounded))
    (Variables|Default|SetTargetLocation (+ Direction (Variables|Default|GetTargetLocation)))
    (Character|LaunchCharacter (Math|Vector|MakeVector 0.0 0.0 (Variables|Default|GetJumpForce)) false true)))

(fn UpdateGrounded
  (Variables|Default|SetIsGrounded (AI|Components|NavMovement|IsMovingonGround (Variables|Character|GetCharacterMovement))))

(fn AddScore
  (params (Score :type Integer))
  (bind _output_get (Variables|Default|SetScoreCount (+ Score (Variables|Default|GetScoreCount))))
  (Default|UpdateScore (Variables|Default|GetScoreUI) _output_get))

(fn AddCoins
  (params (Coins :type Integer))
  (bind _output_get (Variables|Default|SetCoinCount (+ Coins (Variables|Default|GetCoinCount))))
  (Default|UpdateCoins (Variables|Default|GetScoreUI) _output_get))